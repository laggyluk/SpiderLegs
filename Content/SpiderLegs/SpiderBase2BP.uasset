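; Spider base character with procedurally animated legs and a body that tilts to the ground.
; At BeginPlay it gathers child leg meshes' anim instances through ISpiderInterface, ordered by numeric tags.
; Each tick, legs step to velocity-led, downward-traced targets unless the previous leg is moving, sending sine-lifted, interpolated positions to their anim instances.
; The body mesh rotates toward a plane normal summed from all leg targets.
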(event EventBeginPlay
  (bind _legtargets (Variables|Default|GetLegTargets))
  (bind _returnvalue (Utilities|Array|Length _legtargets))
  ;[1 1 1] BeginPlay - setup
  (bind _result (CallFunction|SortLegsbyTag))
  (bind _output_get (Variables|Default|SetLegsAnimRef _result))
  (for _array_element _output_get
    (Utilities|Array|Add (Variables|Default|GetLegInitialTargets) (+ (* (Math|Vector|GetForwardVector (Class|AnimInstance|GetOwningComponent _array_element)) (Variables|Default|GetPosture)) (Variables|/Script/Engine.SceneComponent|GetRelativeLocation (Class|AnimInstance|GetOwningComponent _array_element))))
    (Utilities|Array|Add (Variables|Default|GetLegTargets) (+ (* (Math|Vector|GetForwardVector (Class|AnimInstance|GetOwningComponent _array_element)) (Variables|Default|GetPosture)) (Variables|/Script/Engine.SceneComponent|GetRelativeLocation (Class|AnimInstance|GetOwningComponent _array_element))))
    (Class|ISpiderInterface|SetInitialized(Message) _array_element true)
    (Utilities|Array|Add (Variables|Default|GetStepLengths) (Math|Float|Power (Variables|Default|GetLegReach) 2.0)))
  (Variables|Default|SetCastDownDistance (* (Variables|/Script/Engine.CapsuleComponent|GetCapsuleHalfHeight (Variables|Collision|GetCapsuleComponent)) 2.0))
  (Utilities|Array|Resize (Variables|Default|GetLegCurrentPos) _returnvalue)
  (Utilities|Array|Resize (Variables|Default|GetLegIsMoving) _returnvalue))

(event EventTick
  (params (DeltaSeconds :type Float%20%28single-precision%29))
  ;[1 1 1] tick
  (CallFunction|UpdateLegs false)
  (CallFunction|CalculateBodyAngle)
  (Transformation|SetWorldRotation (Variables|Default|GetArrow1) (Pawn|GetDesiredRotation (Pawn|GetController)) false false))

(fn ConstructionScript)

(fn UpdateLegs
  (params (DebugDraw :type Boolean))
  (bind _legismoving (Variables|Default|GetLegIsMoving))
  (bind _legismoving_2 (Variables|Default|GetLegIsMoving))
  (for (_ _array_index) (Variables|Default|GetLegTargets)
    (bind _output_get (LocalVariables|SettempLoc (+ (Math|Vector|RotateVector (Utilities|Array|Get(acopy) (Variables|Default|GetLegInitialTargets) _array_index) (Math|Rotator|MakeRotator 0.0 0.0 (.yaw (Transformation|GetActorRotation)))) (Transformation|GetActorLocation) (* (Math|Vector|Normalize (Transformation|GetVelocity)) (Variables|Default|GetLegReach)))))
    (if (and (not (Utilities|Array|Get(acopy) _legismoving_2 (Math|Integer|Absolute(Integer) (Math|Integer|%(Integer) (+ _array_index -1) (Utilities|Array|Length _legismoving_2))))) (>= (Math|Vector|VectorLengthXY (- (+ (Math|Vector|RotateVector (Utilities|Array|Get(acopy) (Variables|Default|GetLegInitialTargets) _array_index) (Math|Rotator|MakeRotator 0.0 0.0 (.yaw (Transformation|GetActorRotation)))) (Transformation|GetActorLocation) (* (Math|Vector|Normalize (Transformation|GetVelocity)) (Variables|Default|GetLegReach))) (Utilities|Array|Get(acopy) (Variables|Default|GetLegTargets) _array_index))) (* (Variables|Default|GetLegReach) 1.5))) ; should find next leg position?
      (bind _outhit (Collision|LineTraceByChannel _output_get (- _output_get (Math|Vector|MakeVector 0.0 0.0 (Variables|Default|GetCastDownDistance))) "TraceTypeQuery1" false 0 "None")) ; find ground beneath\nstart from feet location at body level
      (Utilities|Array|SetArrayElem (Variables|Default|GetLegIsMoving) _array_index true)
      (if DebugDraw
        (Rendering|Debug|DrawDebugSphere (.Location (Collision|BreakHitResult _outhit)) 5e+01 8 "(R=1.000000,G=0.003265,B=0.076947,A=1.000000)" 0.5))
      (Utilities|Array|SetArrayElem (Variables|Default|GetStepLengths) _array_index (Math|Float|Clamp(Float) (Math|Vector|VectorLengthSquared (- (Utilities|Array|Get(acopy) (Variables|Default|GetLegTargets) _array_index) (.Location (Collision|BreakHitResult _outhit)))) 0.01 7.766279436516721e+18)) ; cache step length
      (Utilities|Array|SetArrayElem (Variables|Default|GetLegTargets) _array_index (.Location (Collision|BreakHitResult _outhit)))
      (else
        (bind _output_get_2 (LocalVariables|SettempLoc (Math|Interpolation|VInterpTo (Utilities|Array|Get(acopy) (Variables|Default|GetLegCurrentPos) _array_index) (+ (Math|Vector|MakeVector 0.0 0.0 (* (Math|Trig|Sin(Radians) (/ (Math|Vector|VectorLengthSquared (- (Utilities|Array|Get(acopy) (Variables|Default|GetLegCurrentPos) _array_index) (Utilities|Array|Get(acopy) (Variables|Default|GetLegTargets) _array_index))) (Utilities|Array|Get(acopy) (Variables|Default|GetStepLengths) _array_index))) (Variables|Default|GetLegRaise))) (Utilities|Array|Get(acopy) (Variables|Default|GetLegTargets) _array_index)) (Utilities|Time|GetWorldDeltaSeconds) (+ (Variables|Default|GetLegSpeed) (/ (Math|Vector|VectorLength (Transformation|GetVelocity)) 1e+02)))))
        (Utilities|Array|SetArrayElem (Variables|Default|GetLegCurrentPos) _array_index _output_get_2)
        (Class|ISpiderInterface|SetLegTarget(Message) (Utilities|Array|Get(acopy) (Variables|Default|GetLegsAnimRef) _array_index) _output_get_2)
        (if (and (Utilities|Array|Get(acopy) _legismoving _array_index) (<= (/ (Math|Vector|VectorLengthSquared (- (Utilities|Array|Get(acopy) (Variables|Default|GetLegCurrentPos) _array_index) (Utilities|Array|Get(acopy) (Variables|Default|GetLegTargets) _array_index))) (Utilities|Array|Get(acopy) (Variables|Default|GetStepLengths) _array_index)) 0.01))
          (Utilities|Array|SetArrayElem _legismoving _array_index false) ; leg is moving so not on ground
        )))))

(fn CalculateBodyAngle
  (bind _legtargets (Variables|Default|GetLegTargets))
  (if (> (Variables|Default|GetBodyGroundAlignSpeed) 0.0)
    (for (_array_element _array_index) _legtargets
      (LocalVariables|SetplaneNormal (+ (LocalVariables|GetplaneNormal) (Math|Vector|MakeVector (* (- (.Y (Math|Vector|BreakVector _array_element)) (.y (Utilities|Array|Get(acopy) _legtargets (Math|Integer|%(Integer) (+ _array_index 1) (Utilities|Array|Length _legtargets))))) (+ (.Z (Math|Vector|BreakVector _array_element)) (.z (Utilities|Array|Get(acopy) _legtargets (Math|Integer|%(Integer) (+ _array_index 1) (Utilities|Array|Length _legtargets)))))) (* (- (.Z (Math|Vector|BreakVector _array_element)) (.z (Utilities|Array|Get(acopy) _legtargets (Math|Integer|%(Integer) (+ _array_index 1) (Utilities|Array|Length _legtargets))))) (+ (.X (Math|Vector|BreakVector _array_element)) (.x (Utilities|Array|Get(acopy) _legtargets (Math|Integer|%(Integer) (+ _array_index 1) (Utilities|Array|Length _legtargets)))))) (* (- (.X (Math|Vector|BreakVector _array_element)) (.x (Utilities|Array|Get(acopy) _legtargets (Math|Integer|%(Integer) (+ _array_index 1) (Utilities|Array|Length _legtargets))))) (+ (.Y (Math|Vector|BreakVector _array_element)) (.y (Utilities|Array|Get(acopy) _legtargets (Math|Integer|%(Integer) (+ _array_index 1) (Utilities|Array|Length _legtargets))))))))) ; calculate surface normal from leg positions\nhttps://stackoverflow.com/a/2690931/2017839
    )
    (LocalVariables|SetplaneNormal (Math|Vector|Normalize (LocalVariables|GetplaneNormal)))
    (Transformation|SetWorldRotation (Variables|Character|GetMesh) (Math|Interpolation|RInterpTo (Transformation|GetWorldRotation (Variables|Character|GetMesh)) (Math|Conversions|RotationFromXVector (Math|Vector|CrossProduct (Transformation|GetActorRightVector) (LocalVariables|GetplaneNormal))) (Utilities|Time|GetWorldDeltaSeconds) (Variables|Default|GetBodyGroundAlignSpeed)) false false) ; set body rotation
  ))

(fn SortLegsbyTag
  (bind _temparray (LocalVariables|GettempArray))
  (for _array_element (Components|GetChildrenComponents (Variables|Character|GetMesh) false)
    (bind _asskeletal_mesh_component (Utilities|Casting|CastToSkeletalMeshComponent _array_element))
    (if (Utilities|DoesObjectImplementInterface (Components|SkeletalMesh|GetAnimInstance _asskeletal_mesh_component) "/Game/SpiderLegs/ISpiderInterface.ISpiderInterface_C")
      (Utilities|Array|Add (LocalVariables|GettempArray) (Components|SkeletalMesh|GetAnimInstance _asskeletal_mesh_component))))
  (for _index (range 0 (- (Utilities|Array|Length _temparray) 1))
    (for _array_element_2 _temparray
      (if (Components|ComponentHasTag (Class|AnimInstance|GetOwningComponent _array_element_2) (Utilities|String|StringToName (Utilities|String|ToString(Integer) (LocalVariables|Getindex))))
        (Math|Integer|IncrementInt (LocalVariables|Getindex)
          (:%20%20
            (Utilities|Array|Add (LocalVariables|GetResultt) _array_element_2))))))
  (return (LocalVariables|GetResultt)))